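; BP_GameBall is a ball actor that players pick up and that scores on goals.
; On character overlap, HandlePlayerHit shows the hidden HasBallIndicator and destroys the ball, first requiring a zero pickup cooldown if the game mode enables it.
; Hit events, and overlaps with non-characters, share a goal check casting the Hit event's Other to BP_Goal.
; A goal prints its name and increments player 0's Score, leaving the ball alive.
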(event `self.Sphere.OnComponentBeginOverlap`
  (params (OverlappedComponent :type "PrimitiveComponent Object Reference") (OtherActor :type "Actor Object Reference") (OtherComp :type "PrimitiveComponent Object Reference") (OtherBodyIndex :type Integer) (bFromSweep :type Boolean) (SweepResult :type "HitResult Structure (by ref)"))
  (bind _asbp_third_person_character (cast `/Game/Blueprints/Characters/Player/BP_ThirdPersonCharacter` OtherActor)
    (:`then`
      (`self.HandlePlayerHit` _asbp_third_person_character))
    (:`CastFailed`
      (bind _asbp_goal (cast `/Game/Blueprints/NewFolder/BP_Goal` (stale `self.ReceiveHit` Other) :!label _label))
      (`KismetSystemLibrary.PrintString` (`KismetSystemLibrary.GetDisplayName` _asbp_goal))
      (bind _asbp_third_person_character_2 (cast `/Game/Blueprints/Characters/Player/BP_ThirdPersonCharacter` (`GameplayStatics.GetPlayerCharacter` 0)))
      (bind _result (`/Engine/EditorBlueprintResources/StandardMacros.IncrementInt` (`/Game/Blueprints/Characters/Player/BP_ThirdPersonCharacter.Score` _asbp_third_person_character_2))
        (:`  `
          (set `/Game/Blueprints/Characters/Player/BP_ThirdPersonCharacter.Score` _result _asbp_third_person_character_2))))))

(event `self.ReceiveHit`
  (params (MyComp :type "PrimitiveComponent Object Reference") (Other :type "Actor Object Reference") (OtherComp :type "PrimitiveComponent Object Reference") (bSelfMoved :type Boolean) (HitLocation :type "Vector Structure") (HitNormal :type "Vector Structure") (NormalImpulse :type "Vector Structure") (Hit :type "HitResult Structure (by ref)"))
  (goto _label))

(fn `HandlePlayerHit`
  (params (PlayerCharacter :type "/Game/Blueprints/Characters/Player/BP_ThirdPersonCharacter Object Reference"))
  (bind _hasballindicator (`/Game/Blueprints/Characters/Player/BP_ThirdPersonCharacter.HasBallIndicator` PlayerCharacter))
  (bind _asbp_game_mode_test (cast `/Game/Blueprints/BP_GameModeTest` (`GameplayStatics.GetGameMode`)))
  (if (`/Game/Blueprints/BP_GameModeTest.WithPickUpCD` _asbp_game_mode_test)
    (if (== (`/Game/Blueprints/Characters/Player/BP_ThirdPersonCharacter.PickUpCD_Curr` PlayerCharacter) 0.0)
      (if (not (`SceneComponent.IsVisible` _hasballindicator)) :!label _label
        (`SceneComponent.SetVisibility` _hasballindicator true false)
        (`self.K2_DestroyActor` self)))
    (else
      (goto _label))))

(fn `UserConstructionScript`)