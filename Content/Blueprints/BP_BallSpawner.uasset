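; BP_BallSpawner is an actor that spawns a BP_GameBall at its BallSpawnPoint component when play begins.
; The RespawnBall custom event spawns the ball with that point's location and rotation, then turns on physics simulation on its mesh.
; The SpawnBall input action only prints a debug "Hello", as a second RespawnBall call sits unconnected and never runs.
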(event `self.ReceiveBeginPlay`
  (`self.RespawnBall`))

(event `RespawnBall`
  (bind _returnvalue (`|SpawnActorFromClass` "/Game/Blueprints/BP_GameBall.BP_GameBall_C" (`KismetMathLibrary.MakeTransform` (.location (`SceneComponent.K2_GetComponentToWorld` (`self.BallSpawnPoint`))) (.rotation (`SceneComponent.K2_GetComponentToWorld` (`self.BallSpawnPoint`)))) "Undefined" "OverrideRootScale" null null))
  (`PrimitiveComponent.SetSimulatePhysics` (`/Game/Blueprints/BP_GameBall.GameBallMesh` _returnvalue) true))

(event `InputAction|SpawnBall`
  (params (Key :type "Key Structure"))
  (:`Pressed`
    (`KismetSystemLibrary.PrintString` "Hello" :!label _label)))

(event `InputAction|SpawnBall`
  (params (Key :type "Key Structure"))
  (:`Pressed`
    (goto _label)))

(fn `UserConstructionScript`)